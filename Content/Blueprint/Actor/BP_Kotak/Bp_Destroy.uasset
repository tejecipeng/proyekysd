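; Box actor, apparently destructible, with a health value shown through a WB_AIHealthBar widget component.
; On BeginPlay it sets starting Health and seeds the widget's maximum and current values from it.
; A separate UpdateHealthbar function pushes current Health to the widget, but nothing in this file calls it.
; Box1 overlaps pass the other actor to Interact, whose logic is not defined here, as is any damage or destruction handling.
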(event OnComponentBeginOverlap(Box1)
  (params (OverlappedComponent :type Primitive%20Component%20Object%20Reference) (OtherActor :type Actor%20Object%20Reference) (OtherComp :type Primitive%20Component%20Object%20Reference) (OtherBodyIndex :type Integer) (bFromSweep :type Boolean) (SweepResult :type Hit%20Result%20Structure%20%28by%20ref%29))
  (CallFunction|Interact OtherActor))

(event EventBeginPlay
  (|CallParentFunction)
  (Variables|Default|SetHealth 1.5e+02)
  (CallFunction|UpdateMaxHealthBar))

(event Collision|EventActorBeginOverlap
  (params (OtherActor :type Actor%20Object%20Reference))
  (|CallParentFunction OtherActor))

(event EventTick
  (params (DeltaSeconds :type Float%20%28single-precision%29))
  (|CallParentFunction DeltaSeconds) ; This node is disabled and will not be called.\nDrag off pins to build functionality.
)

(fn ConstructionScript
  (|CallParentFunction))

(fn UpdateHealthbar
  (bind _aswb_aihealth_bar (Utilities|Casting|CastToWB_AIHealthBar (UserInterface|GetUserWidgetObject (Variables|Default|GetHealthBar))))
  (Variables|/Game/Blueprint/Actor/BP_Kotak/WB_AIHealthBar.WB_AIHealthBar_C|SetHealth _aswb_aihealth_bar (Variables|Default|GetHealth))
  (return))

(fn UpdateMaxHealthBar
  (bind _aswb_aihealth_bar (Utilities|Casting|CastToWB_AIHealthBar (UserInterface|GetUserWidgetObject (Variables|Default|GetHealthBar))))
  (Variables|/Game/Blueprint/Actor/BP_Kotak/WB_AIHealthBar.WB_AIHealthBar_C|SetMaxHealth _aswb_aihealth_bar (Variables|Default|GetHealth))
  (Variables|/Game/Blueprint/Actor/BP_Kotak/WB_AIHealthBar.WB_AIHealthBar_C|SetHealth _aswb_aihealth_bar (Variables|Default|GetHealth))
  (return))