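; Bp_GlassBox is a destructible glass box that takes damage only from glass bullets.
; BeginPlay calls the parent, sets Health and updates the max health bar.
; Interact casts the incoming actor: a BP_GlassBullet subtracts its Damage, refreshes the health bar, prints Health and destroys the box at zero or below.
; Glass bullets are destroyed on hit, as are BP_peluru bullets, which deal no damage.
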(event EventBeginPlay
  (|CallParentFunction)
  (Variables|Default|SetHealth 5e+01)
  (CallFunction|UpdateMaxHealthBar))

(event Collision|EventActorBeginOverlap
  (params (OtherActor :type Actor%20Object%20Reference))
  (|CallParentFunction OtherActor) ; This node is disabled and will not be called.\nDrag off pins to build functionality.
)

(event EventTick
  (params (DeltaSeconds :type Float%20%28single-precision%29))
  (|CallParentFunction DeltaSeconds) ; This node is disabled and will not be called.\nDrag off pins to build functionality.
)

(event EventInteract
  (params (Actor :type Actor%20Object%20Reference))
  (bind _asbp_glass_bullet (Utilities|Casting|CastToBP_GlassBullet Actor)
    (:then
      (Utilities|FlowControl|Sequence
        (:then_0
          (Variables|Default|SetHealth (- (Variables|Default|GetHealth) (Variables|/Game/Blueprint/Peluru/BP_peluru.BP_peluru_C|GetDamage _asbp_glass_bullet)))
          (CallFunction|UpdateHealthBar)
          (Development|PrintString (Utilities|String|ToString(Float) (Variables|Default|GetHealth)))
          (if (<= (Variables|Default|GetHealth) 0.0)
            (Variables|Default|SetisDead true)
            (Actor|DestroyActor)))
        (:then_1
          (Actor|DestroyActor _asbp_glass_bullet))))
    (:CastFailed
      (bind _asbp_peluru (Utilities|Casting|CastToBP_peluru Actor))
      (Actor|DestroyActor _asbp_peluru))))

(fn ConstructionScript
  (|CallParentFunction))