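; Bp_IronBox is a destructible iron box with a health bar that only iron bullets can damage.
; On BeginPlay it sets its health and updates the maximum on the inherited health bar.
; Its Interact event subtracts a Bp_PeluruIron's damage, updates the bar and destroys the box at zero health.
; Both iron bullets and regular BP_peluru bullets are destroyed on interaction, but regular ones deal no damage.
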(event EventBeginPlay
  (|CallParentFunction)
  (Variables|Default|SetHealth 1.5e+02)
  (CallFunction|UpdateMaxHealthBar))

(event Collision|EventActorBeginOverlap
  (params (OtherActor :type Actor%20Object%20Reference))
  (|CallParentFunction OtherActor) ; This node is disabled and will not be called.\nDrag off pins to build functionality.
)

(event EventTick
  (params (DeltaSeconds :type Float%20%28single-precision%29))
  (|CallParentFunction DeltaSeconds) ; This node is disabled and will not be called.\nDrag off pins to build functionality.
)

(event EventInteract
  (params (Actor :type Actor%20Object%20Reference))
  (bind _asbp_peluru_iron (Utilities|Casting|CastToBp_PeluruIron Actor)
    (:then
      (Utilities|FlowControl|Sequence
        (:then_0
          (Variables|Default|SetHealth (- (Variables|Default|GetHealth) (Variables|/Game/Blueprint/Peluru/BP_peluru.BP_peluru_C|GetDamage _asbp_peluru_iron)))
          (CallFunction|UpdateHealthBar)
          (if (<= (Variables|Default|GetHealth) 0.0)
            (Variables|Default|SetisDead true)
            (Actor|DestroyActor)))
        (:then_1
          (Actor|DestroyActor _asbp_peluru_iron))))
    (:CastFailed
      (bind _asbp_peluru (Utilities|Casting|CastToBP_peluru Actor))
      (Actor|DestroyActor _asbp_peluru))))

(fn ConstructionScript
  (|CallParentFunction))