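; Pushable box actor that slides along one world axis when hit by a BP_PushBullet.
; Box1 overlaps call Interact, which compares the X and Y of the player's Arrow1 forward vector to pick the dominant axis.
; It plays a dragging sound, makes a swept move scaled by that component and destroys the bullet.
; Other overlapping actors are destroyed, except Bp_Character and Bp_Box.
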(event OnComponentBeginOverlap(Box1)
  (params (OverlappedComponent :type Primitive%20Component%20Object%20Reference) (OtherActor :type Actor%20Object%20Reference) (OtherComp :type Primitive%20Component%20Object%20Reference) (OtherBodyIndex :type Integer) (bFromSweep :type Boolean) (SweepResult :type Hit%20Result%20Structure%20%28by%20ref%29))
  (CallFunction|Interact OtherActor))

(event EventBeginPlay
  (|CallParentFunction) ; This node is disabled and will not be called.\nDrag off pins to build functionality.
)

(event Collision|EventActorBeginOverlap
  (params (OtherActor :type Actor%20Object%20Reference))
  (|CallParentFunction OtherActor) ; This node is disabled and will not be called.\nDrag off pins to build functionality.
)

(event EventTick
  (params (DeltaSeconds :type Float%20%28single-precision%29))
  (|CallParentFunction DeltaSeconds))

(event EventInteract
  (params (Actor :type Actor%20Object%20Reference))
  (bind _returnvalue (Transformation|GetActorLocation))
  (bind _asbp_character (Utilities|Casting|CastToBp_Character (Game|GetPlayerCharacter 0)))
  (bind _asbp_push_bullet (Utilities|Casting|CastToBP_PushBullet Actor)
    (:then
      (Audio|PlaySoundatLocation "/Game/Assets/Sound_Bgm/LBFCQTN-box-dragging__mp3cut__mp3cut_net_.LBFCQTN-box-dragging__mp3cut__mp3cut_net_" (Math|Vector|MakeVector (.x _returnvalue) (+ (* (.y (Math|Vector|GetForwardVector (Variables|/Game/Blueprint/char/Bp_Character.Bp_Character_C|GetArrow1 _asbp_character))) 1e+02) (.y _returnvalue)) (.z _returnvalue)) "0, 0, 0" 1.0 1.0 0.0 0 0 0 0)
      (if (< (Math|Float|Absolute(Float) (.x (Math|Vector|GetForwardVector (Variables|/Game/Blueprint/char/Bp_Character.Bp_Character_C|GetArrow1 _asbp_character)))) (Math|Float|Absolute(Float) (.y (Math|Vector|GetForwardVector (Variables|/Game/Blueprint/char/Bp_Character.Bp_Character_C|GetArrow1 _asbp_character)))))
        (Transformation|SetActorLocation (Math|Vector|MakeVector (.x _returnvalue) (+ (* (.y (Math|Vector|GetForwardVector (Variables|/Game/Blueprint/char/Bp_Character.Bp_Character_C|GetArrow1 _asbp_character))) 1e+02) (.y _returnvalue)) (.z _returnvalue)) true false)
        (Utilities|IsValid _asbp_push_bullet
          (:Is%20Valid
            (Actor|DestroyActor _asbp_push_bullet)))
        (else
          (Transformation|SetActorLocation (Math|Vector|MakeVector (+ (* (.x (Math|Vector|GetForwardVector (Variables|/Game/Blueprint/char/Bp_Character.Bp_Character_C|GetArrow1 _asbp_character))) 1e+02) (.x _returnvalue)) (.y _returnvalue) (.z _returnvalue)) true false)
          (Utilities|IsValid _asbp_push_bullet
            (:Is%20Valid
              (Actor|DestroyActor _asbp_push_bullet))))))
    (:CastFailed
      (Utilities|Casting|CastToBp_Character Actor
        (:CastFailed
          (Utilities|Casting|CastToBp_Box Actor
            (:CastFailed
              (Actor|DestroyActor Actor))))))))

(fn ConstructionScript
  (|CallParentFunction))