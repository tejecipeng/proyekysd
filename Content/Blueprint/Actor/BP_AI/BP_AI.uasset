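; BP_AI runs Dijkstra's shortest-path search on a fixed nine-node weighted graph at BeginPlay, from node 0 to node 8.
; Djikstra relaxes edges from an adjacency matrix built as an array of row structs, recording Distance and Previous.
; MinDistance picks each node, returning from inside its loop at the first qualifying unvisited one.
; The route is traced back through Previous, and ReversedPath and total distance are only printed, with no movement.
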(event EventBeginPlay
  (CallFunction|Djikstra 0 8))

(event Collision|EventActorBeginOverlap
  (params (OtherActor :type Actor%20Object%20Reference)))

(event EventTick
  (params (DeltaSeconds :type Float%20%28single-precision%29)))

(fn ConstructionScript)

(fn MinDistance
  (params (distance :type Array%20of%20Integers) (visited :type Array%20of%20Booleans))
  (for _index (range 0 8)
    (if (not (Utilities|Array|Get(acopy) visited _index))
      (if (<= (Utilities|Array|Get(acopy) distance _index) (Variables|Default|GetMinDistance))
        (Variables|Default|SetMinDistance (Utilities|Array|Get(acopy) distance _index))
        (bind _output_get (Variables|Default|SetMinIndex _index))
        (return _output_get)))))

(fn Djikstra
  (params (Start :type Integer) (Target :type Integer))
  (bind _visited (Variables|Default|Getvisited))
  (Variables|Default|SetTarget Target)
  (if (not (or (< Start 0) (>= Start 9)))
    (Utilities|Array|SetArrayElem (Variables|Default|Getdistance) Start 0)
    (for _index (range 0 7)
      (bind _minindex (CallFunction|MinDistance (Variables|Default|Getdistance) _visited))
      (bind _output_get (Variables|Default|SetPointerUh _minindex))
      (Utilities|Array|SetArrayElem _visited _output_get true)
      (for _index_2 (range 0 8)
        (Development|PrintString (Utilities|String|ToString(Integer) _index_2))
        (Variables|Default|SetPointerVeh _index_2)
        (if (not (Utilities|Array|Get(acopy) (Variables|Default|Getvisited) _index_2))
          (if (!= (Utilities|Array|Get(acopy) (.dataarray2d (Utilities|Array|Get(acopy) (Variables|Default|GetadjMatrix) (Variables|Default|GetPointerUh))) (Variables|Default|GetPointerVeh)) 0)
            (if (and (!= (Utilities|Array|Get(acopy) (Variables|Default|Getdistance) (Variables|Default|GetPointerUh)) 2147483647) (< (+ (Utilities|Array|Get(acopy) (Variables|Default|Getdistance) (Variables|Default|GetPointerUh)) (Utilities|Array|Get(acopy) (.dataarray2d (Utilities|Array|Get(acopy) (Variables|Default|GetadjMatrix) (Variables|Default|GetPointerUh))) (Variables|Default|GetPointerVeh))) (Utilities|Array|Get(acopy) (Variables|Default|Getdistance) (Variables|Default|GetPointerVeh))))
              (Utilities|Array|SetArrayElem (Variables|Default|Getdistance) (Variables|Default|GetPointerVeh) (+ (Utilities|Array|Get(acopy) (Variables|Default|Getdistance) (Variables|Default|GetPointerUh)) (Utilities|Array|Get(acopy) (.dataarray2d (Utilities|Array|Get(acopy) (Variables|Default|GetadjMatrix) (Variables|Default|GetPointerUh))) (Variables|Default|GetPointerVeh))))
              (Utilities|Array|SetArrayElem (Variables|Default|Getprevious) (Variables|Default|GetPointerVeh) (Variables|Default|GetPointerUh)))))))
    (if (not (== (Utilities|Array|Get(acopy) (Variables|Default|Getdistance) Target) 2147483647))
      (bind _output_get_2 (Variables|Default|SetCurrent Target))
      (while (!= _output_get_2 Start)
        (Utilities|Array|Add (Variables|Default|GetPath) (Variables|Default|GetCurrent))
        (Variables|Default|SetCurrent (Utilities|Array|Get(acopy) (Variables|Default|Getprevious) (Variables|Default|GetCurrent))))
      (Utilities|Array|Add (Variables|Default|GetPath) Start)
      (for _index_3 (range 0 (Utilities|Array|LastIndex (Variables|Default|GetReversedPath)))
        (Development|PrintString (Utilities|String|ToString(Integer) (Utilities|Array|Get(acopy) (Variables|Default|GetReversedPath) _index_3))))
      (Development|PrintString (Utilities|String|ToString(Integer) (Utilities|Array|Get(acopy) (Variables|Default|Getdistance) Target))))))

(fn ReversePath
  (params (Path :type Array%20of%20Integers))
  (for _index (range (Utilities|Array|LastIndex Path) 0)
    (Utilities|Array|Add (Variables|Default|GetReversedPath) (Utilities|Array|Get(acopy) (Variables|Default|GetPath) _index)))
  (return (Variables|Default|GetReversedPath)))