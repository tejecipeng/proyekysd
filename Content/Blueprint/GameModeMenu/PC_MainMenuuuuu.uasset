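; Player controller for the main menu that creates and switches between the intro (Awal), main menu, level and save/load widgets.
; On BeginPlay it creates all four widgets, shows the cursor and checks IsLevelFinished on the GlobalSetting game instance.
; A finished level opens the level screen after its LoadGame call; otherwise the intro shows for a short delay before the main menu.
; Custom events expose showing and hiding of each screen.
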(event Custom|Show%20Cursor
  (Variables|Default|SetbShowMouseCursor true))

(event Custom|hide%20save%20load
  ;[1 1 1] display save load game
  (Widget|RemovefromParent (Variables|Default|GetWB%20save%20load)))

(event Custom|Display%20Level
  (bind _wb_level (Variables|Default|GetWB%20Level))
  ;[1 1 1] Menu Level
  (Default|LoadGame _wb_level)
  (UserInterface|Viewport|AddtoViewport _wb_level 0))

(event Custom|Hide%20Main%20Menu
  ;[1 1 1] Display Main Menu
  (Widget|RemovefromParent (Variables|Default|GetWB%20Main%20Menu)))

(event Custom|Display%20Main%20Menu
  ;[1 1 1] Display Main Menu
  (UserInterface|Viewport|AddtoViewport (Variables|Default|GetWB%20Main%20Menu) 0))

(event Custom|Hide%20Level
  ;[1 1 1] Menu Level
  (Widget|RemovefromParent (Variables|Default|GetWB%20Level)))

(event Custom|Display%20Awal
  ;[1 1 1] Dispaly Awal
  (UserInterface|Viewport|AddtoViewport (Variables|Default|GetWB%20Awal) 0))

(event Custom|Hide%20Awal
  ;[1 1 1] Dispaly Awal
  (Widget|RemovefromParent (Variables|Default|GetWB%20Awal)))

(event Custom|display%20save%20load
  ;[1 1 1] display save load game
  (UserInterface|Viewport|AddtoViewport (Variables|Default|GetWB%20save%20load) 0))

(event EventBeginPlay
  ;[1 1 1] Begin Play
  (bind _returnvalue (UserInterface|CreateWidget "/Game/Assets/UI/WB_Awal.WB_Awal_C" self))
  (Variables|Default|SetWB%20Awal _returnvalue)
  (bind _returnvalue_2 (UserInterface|CreateWidget "/Game/Assets/UI/WB_saveLoad.WB_saveLoad_C" self))
  (Variables|Default|SetWB%20save%20load _returnvalue_2)
  (bind _returnvalue_3 (UserInterface|CreateWidget "/Game/Assets/UI/WB_Level.WB_Level_C" self))
  (Variables|Default|SetWB%20Level _returnvalue_3)
  (bind _returnvalue_4 (UserInterface|CreateWidget "/Game/Assets/UI/WB_MainMenu.WB_MainMenu_C" self))
  (Variables|Default|SetWB%20Main%20Menu _returnvalue_4)
  (Variables|Default|SetbShowMouseCursor true)
  (bind _asglobal_setting (Utilities|Casting|CastToGlobalSetting (Game|GetGameInstance)))
  (if (Variables|/Game/Blueprint/GlobalVariable/GlobalSetting.GlobalSetting_C|GetisLevelFinished? _asglobal_setting)
    (CallFunction|DisplayLevel)
    (else
      (CallFunction|DisplayAwal)
      (Utilities|FlowControl|Delay 3.0)
      (CallFunction|HideAwal)
      (CallFunction|DisplayMainMenu))))

(event EventTick
  (params (DeltaSeconds :type Float%20%28single-precision%29)))

(fn ConstructionScript)