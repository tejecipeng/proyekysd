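; AI pawn that computes a Dijkstra route through a level's node graph and walks it.
; An adjacency matrix from DT_Level feeds Djikstra, whose MinDistance returns the first unvisited node rather than the true minimum.
; A looping timer sends AIMoveTo toward the BP_Path actor tagged with the next node and current level, removing nodes on success.
; RunAgain loads another level's matrix, resets the search and recomputes the route.
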(event Custom|MoveToPath
  (bind _reversedpath (Variables|Default|GetReversedPath))
  (if (Variables|Default|GetMove?)
    (bind _outactors (Actor|GetAllActorsOfClass "/Game/Blueprint/BP_Path/BP_Path.BP_Path_C"))
    (for _array_element _outactors
      (if (Math|Boolean|ANDBoolean (== (Utilities|String|ToString(Name) (Utilities|Array|Get(acopy) (Variables|/Script/Engine.Actor|GetTags _array_element))) (Utilities|Array|Get(acopy) (Variables|Default|GetReversedPath))) (== (Utilities|Array|Get(acopy) (Variables|/Script/Engine.Actor|GetTags _array_element) 1) (Utilities|String|ToString(Integer) (Variables|Default|Getlvl))) (== (Utilities|Array|Get(acopy) (Variables|/Script/Engine.Actor|GetTags _array_element) 2) "1"))
        (AI|AIMoveTo self "0, 0, 0" _array_element 5e+01 false
          (:OnSuccess
            (Utilities|Array|RemoveIndex _reversedpath)
            (if (== (Utilities|Array|Length _reversedpath) 0)
              (Variables|Default|SetMove? false))))))))

(event Custom|RunAgain
  (params (Level :type Name) (lvl :type Integer))
  (Variables|Default|Setlvl lvl)
  (Variables|Default|SetLevel Level)
  (bind _returnvalue (Utilities|GetDataTableRow "/Game/Blueprint/BP_AI/DT_Level.DT_Level" (Variables|Default|GetLevel))
    (:then
      (Variables|Default|SetadjMatrix (.Path_ (Utilities|Struct|BreakS_Level _returnvalue)))
      (CallFunction|ResetDjikstra)
      (CallFunction|Djikstra 0 (Utilities|Array|LastIndex (Variables|Default|GetadjMatrix))))))

(event Custom|ResetDjikstra
  (bind _distance (Variables|Default|Getdistance))
  (bind _visited (Variables|Default|Getvisited))
  (bind _previous (Variables|Default|Getprevious))
  (for (_ _array_index) _distance
    (Utilities|Array|SetArrayElem _distance _array_index 2147483647))
  (for (_ _array_index_2) _visited
    (Utilities|Array|SetArrayElem _visited _array_index_2 false))
  (for (_ _array_index_3) _previous
    (Utilities|Array|SetArrayElem _previous _array_index_3 -1))
  (Utilities|Array|Clear (Variables|Default|GetPath))
  (Utilities|Array|Clear (Variables|Default|GetReversedPath)))

(event EventBeginPlay
  (bind _returnvalue (Utilities|GetDataTableRow "/Game/Blueprint/BP_AI/DT_Level.DT_Level" "Level1")
    (:then
      (Variables|Default|SetadjMatrix (.Path_ (Utilities|Struct|BreakS_Level _returnvalue)))
      (CallFunction|Djikstra 0 (Utilities|Array|LastIndex (Variables|Default|GetadjMatrix)))
      (Utilities|Time|SetTimerbyEvent (delegate Custom|MoveToPath) 2.0 true))))

(event EventTick
  (params (DeltaSeconds :type Float%20%28single-precision%29)))

(fn ConstructionScript)

(fn MinDistance
  (params (distance :type Array%20of%20Integers) (visited :type Array%20of%20Booleans))
  (Variables|Default|SetMinDistance 2147483647)
  (for _index (range 0 (Utilities|Array|LastIndex (Variables|Default|GetadjMatrix)))
    (if (not (Utilities|Array|Get(acopy) visited _index))
      (if (<= (Utilities|Array|Get(acopy) distance _index) (Variables|Default|GetMinDistance))
        (Variables|Default|SetMinDistance (Utilities|Array|Get(acopy) distance _index))
        (bind _output_get (Variables|Default|SetMinIndex _index))
        (return _output_get)))))

(fn Djikstra
  (params (Start :type Integer) (Target :type Integer))
  (bind _visited (Variables|Default|Getvisited))
  (Variables|Default|SetTarget Target)
  (if (not (or (< Start 0) (>= Start (Utilities|Array|Length (Variables|Default|GetadjMatrix)))))
    (Utilities|Array|SetArrayElem (Variables|Default|Getdistance) Start 0)
    (for _index (range 0 (- (Utilities|Array|LastIndex (Variables|Default|GetadjMatrix)) 1))
      (bind _minindex (CallFunction|MinDistance (Variables|Default|Getdistance) _visited))
      (bind _output_get (Variables|Default|SetPointerUh _minindex))
      (Utilities|Array|SetArrayElem _visited _output_get true)
      (for _index_2 (range 0 (Utilities|Array|LastIndex (Variables|Default|GetadjMatrix)))
        (Variables|Default|SetPointerVeh _index_2)
        (if (not (Utilities|Array|Get(acopy) (Variables|Default|Getvisited) _index_2))
          (if (!= (Utilities|Array|Get(acopy) (.dataarray2d (Utilities|Array|Get(acopy) (Variables|Default|GetadjMatrix) (Variables|Default|GetPointerUh))) (Variables|Default|GetPointerVeh)) 0)
            (if (and (!= (Utilities|Array|Get(acopy) (Variables|Default|Getdistance) (Variables|Default|GetPointerUh)) 2147483647) (< (+ (Utilities|Array|Get(acopy) (Variables|Default|Getdistance) (Variables|Default|GetPointerUh)) (Utilities|Array|Get(acopy) (.dataarray2d (Utilities|Array|Get(acopy) (Variables|Default|GetadjMatrix) (Variables|Default|GetPointerUh))) (Variables|Default|GetPointerVeh))) (Utilities|Array|Get(acopy) (Variables|Default|Getdistance) (Variables|Default|GetPointerVeh))))
              (Utilities|Array|SetArrayElem (Variables|Default|Getdistance) (Variables|Default|GetPointerVeh) (+ (Utilities|Array|Get(acopy) (Variables|Default|Getdistance) (Variables|Default|GetPointerUh)) (Utilities|Array|Get(acopy) (.dataarray2d (Utilities|Array|Get(acopy) (Variables|Default|GetadjMatrix) (Variables|Default|GetPointerUh))) (Variables|Default|GetPointerVeh))))
              (Utilities|Array|SetArrayElem (Variables|Default|Getprevious) (Variables|Default|GetPointerVeh) (Variables|Default|GetPointerUh)))))))
    (if (not (== (Utilities|Array|Get(acopy) (Variables|Default|Getdistance) Target) 2147483647))
      (bind _output_get_2 (Variables|Default|SetCurrent Target))
      (while (!= _output_get_2 Start)
        (Utilities|Array|Add (Variables|Default|GetPath) (Variables|Default|GetCurrent))
        (Variables|Default|SetCurrent (Utilities|Array|Get(acopy) (Variables|Default|Getprevious) (Variables|Default|GetCurrent))))
      (Utilities|Array|Add (Variables|Default|GetPath) Start)
      (bind _reversedpath (CallFunction|ReversePath (Variables|Default|GetPath)))
      (Variables|Default|SetReversedPath _reversedpath)
      (for _index_3 (range 0 (Utilities|Array|LastIndex (Variables|Default|GetReversedPath)))
        _))))

(fn ReversePath
  (params (Path :type Array%20of%20Integers))
  (bind _arrayelement (Utilities|Array|ReverseforEachLoop Path)
    (:LoopBody
      (Utilities|Array|Add (Variables|Default|GetReversedPath) _arrayelement))
    (:Completed
      (return (Variables|Default|GetReversedPath)))))