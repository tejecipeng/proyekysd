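; Gameplay game mode that runs a level countdown and checks whether the player took the same path as the AI.
; BeginPlay briefly waits, then shows the player controller's pause display; Tick uses a one-second Delay to count down minutes and seconds, switching to the lose display at zero.
; The cekbintang event compares BP_AI's ReversedPath to numeric tags on the character's Path, clearing a per-level Short flag on mismatch, then increments CountFinish.
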(event Custom|cek%20bintang
  (bind _returnvalue (Actor|GetActorOfClass "/Game/Blueprint/BP_AI/BP_AI.BP_AI_C"))
  (bind _asbp_character (Utilities|Casting|CastToBp_Character (Game|GetPlayerCharacter 0)))
  (for (_array_element _array_index) (Variables|/Game/Blueprint/BP_AI/BP_AI.BP_AI_C|GetReversedPath _returnvalue)
    (if (not (== _array_element (Math|Conversions|ToInteger(Byte) (Utilities|String|ToString(Name) (Utilities|Array|Get(acopy) (Variables|/Script/Engine.Actor|GetTags (Utilities|Array|Get(acopy) (Variables|/Game/Blueprint/char/Bp_Character.Bp_Character_C|GetPath _asbp_character) _array_index)))))))
      (if (== (Variables|Default|GetcountFinish) 1)
        (Variables|Default|SetShortLv1 false)
        (elif (== (Variables|Default|GetcountFinish) 2)
          (Variables|Default|SetShortLv2 false)
          (else
            (Variables|Default|SetShortLv3 false))))))
  (Math|Integer|IncrementInt (Variables|Default|GetcountFinish)))

(event EventBeginPlay
  (Utilities|FlowControl|Delay 0.1)
  (bind _aspc_player_controller (Utilities|Casting|CastToPC_PlayerController (Game|GetPlayerController 0)))
  (Variables|Default|SetPC_Player _aspc_player_controller)
  (Default|DisplayPause (Variables|Default|GetPC_Player)))

(event EventTick
  (params (DeltaSeconds :type Float%20%28single-precision%29))
  (bind _pc_player (Variables|Default|GetPC_Player))
  (Utilities|FlowControl|Delay 1.0)
  (if (== (Variables|Default|GetSeconds) 0.0)
    (if (== (Variables|Default|GetMinutes) 0.0)
      (Default|HidePause _pc_player)
      (Default|DisplayLose _pc_player)
      (else
        (Variables|Default|SetSeconds 59.0)
        (Variables|Default|SetMinutes (- (Variables|Default|GetMinutes) 1))))
    (else
      (Variables|Default|SetSeconds (- (Variables|Default|GetSeconds) 1.0)))))

(fn ConstructionScript)