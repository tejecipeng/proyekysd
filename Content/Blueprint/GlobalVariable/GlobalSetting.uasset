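; GlobalSetting is a global game object that manages the player's save and level-progress flags.
; On Init it loads the "save game" slot as BP_SaveGame, or creates and saves one if none exists.
; SaveGame writes the Level 2–4 flags to that object and slot, while IsLevel1 is only assigned to itself.
; Newgame overwrites the slot with a fresh save; LoadGame only calls DisplayLevel on the main-menu controller.
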(event Custom|new%20game
  (bind _returnvalue (SaveGame|CreateSaveGameObject "/Game/Blueprint/LoadSaveGame/BP_SaveGame.BP_SaveGame_C"))
  (bind _output_get (Variables|Default|SetSaveGameObject _returnvalue))
  (SaveGame|SaveGametoSlot _output_get "save game"))

(event Custom|LoadGame
  (bind _aspc_main_menuuuuu (Utilities|Casting|CastToPC_MainMenuuuuu (Game|GetPlayerController 0)))
  (Default|DisplayLevel _aspc_main_menuuuuu))

(event Custom|SaveGame
  (bind _savegameobject (Variables|Default|GetSaveGameObject))
  (Variables|Default|SetisLevel1? (Variables|Default|GetisLevel1?))
  (Variables|/Game/Blueprint/LoadSaveGame/BP_SaveGame.BP_SaveGame_C|SetisLevel2? _savegameobject (Variables|Default|GetisLevel2?))
  (Variables|/Game/Blueprint/LoadSaveGame/BP_SaveGame.BP_SaveGame_C|SetisLevel3? _savegameobject (Variables|Default|GetisLevel3?))
  (Variables|/Game/Blueprint/LoadSaveGame/BP_SaveGame.BP_SaveGame_C|SetisLevel4? _savegameobject (Variables|Default|GetisLevel4?))
  (SaveGame|SaveGametoSlot (Variables|Default|GetSaveGameObject) "save game"))

(event EventInit
  (Utilities|FlowControl|Sequence
    (:then_0
      (bind _returnvalue (SaveGame|DoesSaveGameExist "save game"))
      (if _returnvalue
        (bind _returnvalue_2 (SaveGame|LoadGamefromSlot "save game"))
        (bind _asbp_save_game (Utilities|Casting|CastToBP_SaveGame _returnvalue_2))
        (Variables|Default|SetSaveGameObject _asbp_save_game)
        (else
          (bind _returnvalue_3 (SaveGame|CreateSaveGameObject "/Game/Blueprint/LoadSaveGame/BP_SaveGame.BP_SaveGame_C"))
          (bind _output_get (Variables|Default|SetSaveGameObject _returnvalue_3))
          (SaveGame|SaveGametoSlot _output_get "save game"))))))