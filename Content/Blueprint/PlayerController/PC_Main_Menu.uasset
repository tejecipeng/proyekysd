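; Player controller for the main menu that owns and toggles the main menu and play screen widgets.
; On BeginPlay it creates WB_Main_Menu and WB_Play for itself and stores them without showing either.
; Custom events add each widget to the viewport or remove it from its parent, leaving screen switching to callers.
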(event Custom|Display%20Main%20Menu
  (UserInterface|Viewport|AddtoViewport (Variables|Default|GetWB%20Main%20Menu) 0))

(event Custom|Hide%20Main%20Menu
  (Widget|RemovefromParent (Variables|Default|GetWB%20Main%20Menu)))

(event Custom|Display%20Play
  (UserInterface|Viewport|AddtoViewport (Variables|Default|GetWB%20Play) 0))

(event Custom|Hide%20Play
  (Widget|RemovefromParent (Variables|Default|GetWB%20Play)))

(event EventTick
  (params (DeltaSeconds :type Float%20%28single-precision%29)))

(event EventBeginPlay
  (bind _returnvalue (UserInterface|CreateWidget "/Game/UI/WB_Main_Menu.WB_Main_Menu_C" self))
  (Variables|Default|SetWB%20Main%20Menu _returnvalue)
  (bind _returnvalue_2 (UserInterface|CreateWidget "/Game/UI/WB_Play.WB_Play_C" self))
  (Variables|Default|SetWB%20Play _returnvalue_2))

(fn ConstructionScript)