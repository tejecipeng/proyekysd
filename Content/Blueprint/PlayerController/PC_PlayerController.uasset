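; PC_PlayerController is the player controller that manages the game's UI screens: pause, main pause, win, lose and star.
; BeginPlay creates and caches the widgets, except that WBWin is set to None and the WB_MainGame widget is never stored or displayed.
; Display and Hide events add or remove each screen, and ShowCursor enables the mouse cursor.
; CekFinish only casts the player character to Bp_Character, with no further logic.
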(event Custom|Cek%20Finish
  (Utilities|Casting|CastToBp_Character (Game|GetPlayerCharacter 0)))

(event Custom|Show%20Cursor
  (Variables|Default|SetbShowMouseCursor true))

(event Custom|Hide%20Star
  (Widget|RemovefromParent (Variables|Default|GetWB_Star)))

(event Custom|Display%20Main%20Pause
  (UserInterface|Viewport|AddtoViewport (Variables|Default|GetWB%20Main%20Pause) 0))

(event Custom|Hide%20Main%20Pause
  (Widget|RemovefromParent (Variables|Default|GetWB%20Main%20Pause)))

(event Custom|Display%20Pause
  (UserInterface|Viewport|AddtoViewport (Variables|Default|GetWB_Pause) 0))

(event Custom|Hide%20Pause
  (Widget|RemovefromParent (Variables|Default|GetWB_Pause)))

(event Custom|Display%20Win
  (UserInterface|Viewport|AddtoViewport (Variables|Default|GetWB%20Win) 0))

(event Custom|Hide%20Win
  (Widget|RemovefromParent (Variables|Default|GetWB%20Win)))

(event Custom|Display%20Lose
  (UserInterface|Viewport|AddtoViewport (Variables|Default|GetWB%20Lose) 0))

(event Custom|Hide%20Lose
  (Widget|RemovefromParent (Variables|Default|GetWB%20Lose)))

(event Custom|Display%20Star
  (UserInterface|Viewport|AddtoViewport (Variables|Default|GetWB_Star) 0))

(event EventBeginPlay
  (bind _returnvalue (UserInterface|CreateWidget "/Game/UI/WB_Pause.WB_Pause_C" self))
  (Variables|Default|SetWB_Pause _returnvalue)
  (bind _returnvalue_2 (UserInterface|CreateWidget "/Game/UI/WB_Main_Pause.WB_Main_Pause_C" self))
  (Variables|Default|SetWB%20Main%20Pause _returnvalue_2)
  (UserInterface|CreateWidget "/Game/Blueprint/WidgetUI/WB_MainGame.WB_MainGame_C" self)
  (Variables|Default|SetWB%20Win 0)
  (bind _returnvalue_3 (UserInterface|CreateWidget "/Game/UI/WB_Lose.WB_Lose_C" self))
  (Variables|Default|SetWB%20Lose _returnvalue_3)
  (bind _returnvalue_4 (UserInterface|CreateWidget "/Game/UI/WB_Star.WB_Star_C" self))
  (Variables|Default|SetWB_Star _returnvalue_4))

(fn ConstructionScript)