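; Gameplay player controller that owns the level's UI widgets and routes input to Bp_Character.
; BeginPlay creates the widgets, adds the Enhanced Input context and shows pause and bullet-icon UI; events show, hide or update widgets.
; Camera and shoot inputs are gated by IsShoot, while switching cycles bullet classes, skipping unavailable ones.
; Left click traces under the cursor and stores a hit BP_Path in ArrPath.
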(event Custom|Display%20Star
  ;[1 1 1] Display Star
  (UserInterface|Viewport|AddtoViewport (Variables|Default|GetWB%20Star) 0))

(event Custom|Show%20Cursor
  (Variables|Default|SetbShowMouseCursor true))

(event Custom|load%20game
  ;[1 1 1] Load Game
  (Default|LoadGame (Variables|Default|GetWB%20Level)))

(event Custom|Hide%20Pause
  ;[1 1 1] Pause
  (Widget|RemovefromParent (Variables|Default|GetWB%20Pause)))

(event Custom|Display%20Menu%20Pause
  ;[1 1 1] Menu Pause
  (UserInterface|Viewport|AddtoViewport (Variables|Default|GetWB%20Menu%20Pause) 0))

(event Custom|Hide%20Menu%20Pause
  ;[1 1 1] Menu Pause
  (Widget|RemovefromParent (Variables|Default|GetWB%20Menu%20Pause)))

(event Custom|Display%20BulletIcon
  ;[1 1 1] Menu Change Bullet
  (UserInterface|Viewport|AddtoViewport (Variables|Default|GetWB%20BulletIcon) 0))

(event Custom|Display%20Finish
  ;[1 1 1] Finish
  (UserInterface|Viewport|AddtoViewport (Variables|Default|GetWB%20Finish) 0))

(event Custom|Hide%20Finish
  ;[1 1 1] Finish
  (Widget|RemovefromParent (Variables|Default|GetWB%20Finish)))

(event Custom|Hide%20BulletIcon
  ;[1 1 1] Menu Change Bullet
  (Widget|RemovefromParent (Variables|Default|GetWB%20BulletIcon)))

(event Custom|Update%20UI%20Level
  ;[1 1 1] update UI Level
  (bind _returnvalue (Game|GetCurrentLevelName true))
  (Default|UpdateUILevel (Variables|Default|GetWB%20Level) (.RightS (Utilities|String|Split _returnvalue "level"))))

(event Custom|Display%20Level
  ;[1 1 1] Menu Level
  (UserInterface|Viewport|AddtoViewport (Variables|Default|GetWB%20Level) 0))

(event Custom|Hide%20Level
  ;[1 1 1] Menu Level
  (Widget|RemovefromParent (Variables|Default|GetWB%20Level)))

(event Custom|Display%20Pause
  ;[1 1 1] Pause
  (UserInterface|Viewport|AddtoViewport (Variables|Default|GetWB%20Pause) 0))

(event Input|EnhancedActionEvents|EnhancedInputActionIA_Camera
  (params (ActionValue :type Vector%202D%20Structure) (ElapsedSeconds :type Float%20%28double-precision%29) (TriggeredSeconds :type Float%20%28double-precision%29) (InputAction :type Input%20Action%20Object%20Reference :default "/Game/Blueprint/Input/IA_Camera.IA_Camera"))
  ;[1 1 1] char Camera
  (if (not (Variables|/Game/Blueprint/char/Bp_Character.Bp_Character_C|GetisShoot? (Variables|Default|GetOwnCharacter)))
    (Pawn|Input|AddControllerYawInput (Variables|Default|GetOwnCharacter) (* (.x ActionValue) (Variables|Default|Getturn%20rate%20gamepad) (Utilities|Time|GetWorldDeltaSeconds)))
    (Pawn|Input|AddControllerPitchInput (Variables|Default|GetOwnCharacter) (* (.y ActionValue) (Variables|Default|Getturn%20rate%20gamepad) (Utilities|Time|GetWorldDeltaSeconds)))))

(event Input|EnhancedActionEvents|EnhancedInputActionIA_Shoot
  (params (ActionValue :type Boolean) (ElapsedSeconds :type Float%20%28double-precision%29) (TriggeredSeconds :type Float%20%28double-precision%29) (InputAction :type Input%20Action%20Object%20Reference :default "/Game/Blueprint/Input/IA_Shoot.IA_Shoot"))
  ;[1 1 1] Char Shoot
  (:Started
    (if (not (Variables|/Game/Blueprint/char/Bp_Character.Bp_Character_C|GetisShoot? (Variables|Default|GetOwnCharacter)))
      (Variables|/Game/Blueprint/char/Bp_Character.Bp_Character_C|SetisShoot? (Variables|Default|GetOwnCharacter) true))))

(event Input|EnhancedActionEvents|EnhancedInputActionIA_Switch
  (params (ActionValue :type Boolean) (ElapsedSeconds :type Float%20%28double-precision%29) (TriggeredSeconds :type Float%20%28double-precision%29) (InputAction :type Input%20Action%20Object%20Reference :default "/Game/Blueprint/Input/IA_Switch.IA_Switch"))
  (bind _owncharacter (Variables|Default|GetOwnCharacter))
  (bind _bullets (Variables|/Game/Blueprint/char/Bp_Character.Bp_Character_C|GetBullets _owncharacter))
  ;[1 1 1] Switch Bullet
  (:Started
    (Math|Integer|IncrementInt (Variables|/Game/Blueprint/char/Bp_Character.Bp_Character_C|GetChangeBullet _owncharacter) :!label _label
      (:%20%20
        (switch int (Variables|/Game/Blueprint/char/Bp_Character.Bp_Character_C|GetChangeBullet _owncharacter) :!label _label_2
          (:0
            (Variables|/Game/Blueprint/char/Bp_Character.Bp_Character_C|SetPeluru _owncharacter "/Game/Blueprint/Peluru/BP_PushBullet.BP_PushBullet_C"))
          (:1
            (if (Utilities|Array|Get(acopy) _bullets 1)
              (Variables|/Game/Blueprint/char/Bp_Character.Bp_Character_C|SetPeluru _owncharacter "/Game/Blueprint/Peluru/Bp_WoodenBulllet.Bp_WoodenBulllet_C")
              (else
                (goto _label))))
          (:2
            (if (Utilities|Array|Get(acopy) _bullets 2)
              (Variables|/Game/Blueprint/char/Bp_Character.Bp_Character_C|SetPeluru _owncharacter "/Game/Blueprint/Peluru/Bp_PeluruIron.Bp_PeluruIron_C")
              (else
                (goto _label))))
          (:3
            (if (Utilities|Array|Get(acopy) _bullets 3)
              (Variables|/Game/Blueprint/char/Bp_Character.Bp_Character_C|SetPeluru _owncharacter "/Game/Blueprint/Peluru/BP_GlassBullet.BP_GlassBullet_C")
              (Variables|/Game/Blueprint/char/Bp_Character.Bp_Character_C|SetChangeBullet _owncharacter -1)
              (else
                (Variables|/Game/Blueprint/char/Bp_Character.Bp_Character_C|SetChangeBullet _owncharacter 0)
                (goto _label_2)))))))))

(event EventTick
  (params (DeltaSeconds :type Float%20%28single-precision%29)))

(event EventBeginPlay
  (bind _returnvalue (PlayerController|LocalPlayerSubsystems|GetEnhancedInputLocalPlayerSubsystem))
  ;[1 1 1] Begin Play
  (bind _returnvalue_2 (UserInterface|CreateWidget "/Game/Assets/UI/WB_Star.WB_Star_C"))
  (Variables|Default|SetWB%20Star _returnvalue_2)
  (bind _returnvalue_3 (UserInterface|CreateWidget "/Game/Assets/UI/WB_Pause.WB_Pause_C" self))
  (Variables|Default|SetWB%20Pause _returnvalue_3)
  (bind _returnvalue_4 (UserInterface|CreateWidget "/Game/Assets/UI/WB_MenuPause.WB_MenuPause_C" self))
  (Variables|Default|SetWB%20Menu%20Pause _returnvalue_4)
  (Utilities|IsValid _returnvalue
    (:Is%20Valid
      (Input|AddMappingContext _returnvalue "/Game/Blueprint/Input/IMC_Gameplay.IMC_Gameplay" 0 "(bIgnoreAllPressedKeysUntilRelease=True,bForceImmediately=False,bNotifyUserSettings=False)")
      (bind _asbp_character (Utilities|Casting|CastToBp_Character (Game|GetPlayerCharacter 0))
        (:then
          (Variables|Default|SetOwnCharacter _asbp_character)
          (bind _returnvalue_5 (UserInterface|CreateWidget "/Game/Assets/UI/WB_Level.WB_Level_C" self))
          (Variables|Default|SetWB%20Level _returnvalue_5)
          (bind _returnvalue_6 (UserInterface|CreateWidget "/Game/Assets/UI/WB_Finish.WB_Finish_C" self))
          (Variables|Default|SetWB%20Finish _returnvalue_6)
          (bind _returnvalue_7 (UserInterface|CreateWidget "/Game/Assets/UI/WB_ChangBulletIcon.WB_ChangBulletIcon_C" self))
          (Variables|Default|SetWB%20BulletIcon _returnvalue_7)
          (CallFunction|DisplayPause)
          (CallFunction|DisplayBulletIcon))
        (:CastFailed
          (Development|PrintString "aaaa"))))))

(event Input|MouseEvents|LeftMouseButton
  (params (Key :type Key%20Structure :default "None"))
  (bind _returnvalue (Game|GetPlayerController 0))
  (bind _array (Utilities|Array|MakeArray "ObjectTypeQuery1"))
  (bind (_hitresult _returnvalue_2) (Class|PlayerController|GetHitResultUnderCursorforObjects _returnvalue _array true))
  ;[1 1 1] Klik Mouse buat jalan ke path tersebut
  (:Pressed
    (Variables|/Script/Engine.PlayerController|SetbShowMouseCursor _returnvalue true)
    (if _returnvalue_2
      (bind _asbp_path (Utilities|Casting|CastToBP_Path (.HitActor (Collision|BreakHitResult _hitresult))))
      (Variables|Default|SetArrPath (Utilities|Array|MakeArray _asbp_path)))))

(fn ConstructionScript)