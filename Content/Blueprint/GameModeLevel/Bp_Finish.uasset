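; Bp_Finish is a level finish trigger that reacts when a Bp_Box actor overlaps its Box component.
; It caches the PC_PlayerController on BeginPlay, then on overlap has it display stars, show the cursor and update the level UI.
; It also writes the IsLevelFinished field on the GlobalSetting game instance and shows the finish display if the current level is level4.
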(event OnComponentBeginOverlap(Box)
  (params (OverlappedComponent :type Primitive%20Component%20Object%20Reference) (OtherActor :type Actor%20Object%20Reference) (OtherComp :type Primitive%20Component%20Object%20Reference) (OtherBodyIndex :type Integer) (bFromSweep :type Boolean) (SweepResult :type Hit%20Result%20Structure%20%28by%20ref%29))
  (bind _playercontroller (Variables|Default|GetPlayerController))
  (Utilities|Casting|CastToBp_Box OtherActor)
  (Default|DisplayStar _playercontroller)
  (Default|ShowCursor _playercontroller)
  (Default|UpdateUILevel _playercontroller)
  (bind _asglobal_setting (Utilities|Casting|CastToGlobalSetting (Game|GetGameInstance)))
  (Variables|/Game/Blueprint/GlobalVariable/GlobalSetting.GlobalSetting_C|SetisLevelFinished? _asglobal_setting 0 true)
  (bind _returnvalue (Game|GetCurrentLevelName true))
  (if (Utilities|Enum|Equal(Enum) _returnvalue "level4")
    (Default|DisplayFinish (Variables|Default|GetPlayerController))))

(event EventBeginPlay
  (bind _aspc_player_controller (Utilities|Casting|CastToPC_PlayerController (Game|GetPlayerController 0)))
  (Variables|Default|SetPlayerController _aspc_player_controller))

(event Collision|EventActorBeginOverlap
  (params (OtherActor :type Actor%20Object%20Reference)))

(event EventTick
  (params (DeltaSeconds :type Float%20%28single-precision%29)))

(fn ConstructionScript)