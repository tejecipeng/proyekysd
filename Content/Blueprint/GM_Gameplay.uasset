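; Gameplay game mode that alternates player and AI turns across three levels, with a countdown that runs on player turns and shows the lose screen at zero.
; BeginPlay sorts tagged camera pawns into arrays; Tick possesses the one matching the Start counter and swaps the UI.
; Switch events advance Start, reposition both characters at the next level's start and rerun the AI.
; CekBintang compares the player's path to the AI's ReversedPath for end-screen stars.
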(event Custom|cek%20bintang
  ;[1 1 1] Cek bintang untuk tampilan akhir game jika menang --Margareth
  (bind _returnvalue (Actor|GetActorOfClass "/Game/Blueprint/BP_AI/BP_AI.BP_AI_C"))
  (bind _returnvalue_2 (Actor|GetActorOfClass "/Game/Blueprint/char/Bp_Character.Bp_Character_C"))
  (for (_array_element _array_index) (Variables|/Game/Blueprint/BP_AI/BP_AI.BP_AI_C|GetReversedPath _returnvalue)
    (if (not (== _array_element (Math|Conversions|ToInteger(Byte) (Utilities|String|ToString(Name) (Utilities|Array|Get(acopy) (Variables|/Script/Engine.Actor|GetTags (Utilities|Array|Get(acopy) (Variables|/Game/Blueprint/char/Bp_Character.Bp_Character_C|GetPath _returnvalue_2) _array_index)))))))
      (if (== (Variables|Default|GetcountFinish) 1)
        (Variables|Default|SetShortLv1 false)
        (elif (== (Variables|Default|GetcountFinish) 2)
          (Variables|Default|SetShortLv2 false)
          (else
            (Variables|Default|SetShortLv3 false))))))
  (Math|Integer|IncrementInt (Variables|Default|GetcountFinish)))

(event Custom|SwitchPlayerAI
  ;[1 1 1] Event tick (mengatur detikan UI, switch antara player dan AI, dan setting player atau AI ke start di level itu) --Margareth
  (Math|Integer|IncrementInt (Variables|Default|Getstart)
    (:%20%20
      (CallFunction|CekBintang))))

(event Custom|SwitchAIPlayer
  (bind _start (Variables|Default|Getstart))
  (bind _returnvalue (/ _start 2))
  (bind _returnvalue_2 (+ _returnvalue 1))
  ;[1 1 1] Event tick (mengatur detikan UI, switch antara player dan AI, dan setting player atau AI ke start di level itu) --Margareth
  (Utilities|FlowControl|Sequence
    (:then_0
      (Math|Integer|IncrementInt (Variables|Default|Getstart)
        (:%20%20
          (bind _outactors (Actor|GetAllActorsOfClass "/Game/Blueprint/char/Bp_Character.Bp_Character_C"))
          (Default|ResetPlayer (Utilities|Array|Get(acopy) _outactors))
          (bind _outactors_2 (Actor|GetAllActorsOfClass "/Game/Blueprint/BP_AI/BP_AI.BP_AI_C"))
          (if (== _returnvalue_2 2)
            (Default|RunAgain (Utilities|Array|Get(acopy) _outactors_2) "Level2" 2)
            (bind _outactors_3 (Actor|GetAllActorsOfClasswithTag "/Game/Blueprint/BP_Path/BP_Start.BP_Start_C" "1"))
            (Transformation|SetActorLocation (Utilities|Array|Get(acopy) _outactors) (Transformation|GetActorLocation (Utilities|Array|Get(acopy) _outactors_3)) false false)
            (bind _outactors_4 (Actor|GetAllActorsOfClasswithTag "/Game/Blueprint/BP_Path/BP_StartAI.BP_StartAI_C" "1"))
            (Transformation|SetActorLocation (Utilities|Array|Get(acopy) _outactors_2) (Transformation|GetActorLocation (Utilities|Array|Get(acopy) _outactors_4)) false false)
            (elif (== _returnvalue_2 3)
              (Default|RunAgain (Utilities|Array|Get(acopy) _outactors_2) "Level3" 3)
              (bind _outactors_5 (Actor|GetAllActorsOfClasswithTag "/Game/Blueprint/BP_Path/BP_Start.BP_Start_C" "2"))
              (Transformation|SetActorLocation (Utilities|Array|Get(acopy) _outactors) (Transformation|GetActorLocation (Utilities|Array|Get(acopy) _outactors_5)) false false)
              (bind _outactors_6 (Actor|GetAllActorsOfClasswithTag "/Game/Blueprint/BP_Path/BP_StartAI.BP_StartAI_C" "2"))
              (Transformation|SetActorLocation (Utilities|Array|Get(acopy) _outactors_2) (Transformation|GetActorLocation (Utilities|Array|Get(acopy) _outactors_6)) false false))))))))

(event Custom|ShowUIPlayer
  ;[1 1 1] Event tick (mengatur detikan UI, switch antara player dan AI, dan setting player atau AI ke start di level itu) --Margareth
  (bind _aspc_player_controller (Utilities|Casting|CastToPC_PlayerController (Game|GetPlayerController 0)))
  (Default|HideWidgetAI _aspc_player_controller)
  (Default|DisplayPause _aspc_player_controller))

(event Custom|ShowUIAI
  ;[1 1 1] Event tick (mengatur detikan UI, switch antara player dan AI, dan setting player atau AI ke start di level itu) --Margareth
  (bind _aspc_player_controller (Utilities|Casting|CastToPC_PlayerController (Game|GetPlayerController 0)))
  (Default|HidePause _aspc_player_controller)
  (Default|ShowWidgetAI _aspc_player_controller))

(event EventBeginPlay
  (bind _pawncameraai (Variables|Default|GetPawnCameraAI))
  (bind _pawncamera (Variables|Default|GetPawnCamera))
  ;[1 1 1] begin play gameplay --Margareth
  (Utilities|FlowControl|Delay 0.1)
  (Utilities|FlowControl|Sequence
    (:then_0
      (Utilities|Array|Clear _pawncamera)
      (Utilities|Array|Add _pawncamera 0)
      (Utilities|Array|Add _pawncamera 0)
      (Utilities|Array|Add _pawncamera 0)
      (Utilities|Array|Add _pawncameraai 0)
      (Utilities|Array|Add _pawncameraai 0)
      (Utilities|Array|Add _pawncameraai 0)
      (bind _outactors (Actor|GetAllActorsOfClass "/Game/Blueprint/BP_Camera/BP_CameraPlayer.BP_CameraPlayer_C"))
      (for _array_element _outactors
        (if (and (== (Utilities|Array|Get(acopy) (Variables|/Script/Engine.Actor|GetTags _array_element)) "1") (== (Utilities|Array|Get(acopy) (Variables|/Script/Engine.Actor|GetTags _array_element) 1) "Player"))
          (Utilities|Array|SetArrayElem (Variables|Default|GetPawnCamera) 0 _array_element)
          (elif (and (== (Utilities|Array|Get(acopy) (Variables|/Script/Engine.Actor|GetTags _array_element)) "2") (== (Utilities|Array|Get(acopy) (Variables|/Script/Engine.Actor|GetTags _array_element) 1) "Player"))
            (Utilities|Array|SetArrayElem (Variables|Default|GetPawnCamera) 1 _array_element)
            (elif (and (== (Utilities|Array|Get(acopy) (Variables|/Script/Engine.Actor|GetTags _array_element)) "3") (== (Utilities|Array|Get(acopy) (Variables|/Script/Engine.Actor|GetTags _array_element) 1) "Player"))
              (Utilities|Array|SetArrayElem (Variables|Default|GetPawnCamera) 2 _array_element)))))
      (bind _outactors_2 (Actor|GetAllActorsOfClass "/Game/Blueprint/BP_Camera/BP_CameraAI.BP_CameraAI_C"))
      (for _array_element_2 _outactors_2
        (if (and (== (Utilities|Array|Get(acopy) (Variables|/Script/Engine.Actor|GetTags _array_element_2)) "1") (== (Utilities|Array|Get(acopy) (Variables|/Script/Engine.Actor|GetTags _array_element_2) 1) "AI"))
          (Utilities|Array|SetArrayElem (Variables|Default|GetPawnCameraAI) 0 _array_element_2)
          (elif (and (== (Utilities|Array|Get(acopy) (Variables|/Script/Engine.Actor|GetTags _array_element_2)) "2") (== (Utilities|Array|Get(acopy) (Variables|/Script/Engine.Actor|GetTags _array_element_2) 1) "AI"))
            (Utilities|Array|SetArrayElem (Variables|Default|GetPawnCameraAI) 1 _array_element_2)
            (elif (and (== (Utilities|Array|Get(acopy) (Variables|/Script/Engine.Actor|GetTags _array_element_2)) "3") (== (Utilities|Array|Get(acopy) (Variables|/Script/Engine.Actor|GetTags _array_element_2) 1) "AI"))
              (Utilities|Array|SetArrayElem (Variables|Default|GetPawnCameraAI) 2 _array_element_2))))))
    (:then_1
      (bind _aspc_player_controller (Utilities|Casting|CastToPC_PlayerController (Game|GetPlayerController 0)))
      (Variables|Default|SetPC_Player _aspc_player_controller)
      (Default|DisplayPause (Variables|Default|GetPC_Player)))))

(event EventTick
  (params (DeltaSeconds :type Float%20%28single-precision%29))
  (bind _returnvalue (Game|GetPlayerController 0))
  (bind _returnvalue_2 (Game|GetPlayerController 0))
  (bind _returnvalue_3 (Game|GetPlayerController 0))
  (bind _returnvalue_4 (Game|GetPlayerController 0))
  (bind _returnvalue_5 (Game|GetPlayerController 0))
  (bind _returnvalue_6 (Game|GetPlayerController 0))
  (bind _pawncamera (Variables|Default|GetPawnCamera))
  (bind _pawncameraai (Variables|Default|GetPawnCameraAI))
  (bind _pawncamera_2 (Variables|Default|GetPawnCamera))
  (bind _pawncameraai_2 (Variables|Default|GetPawnCameraAI))
  (bind _pawncameraai_3 (Variables|Default|GetPawnCameraAI))
  (bind _pawncamera_3 (Variables|Default|GetPawnCamera))
  (bind _pc_player (Variables|Default|GetPC_Player))
  (bind _output (Utilities|Array|Get(acopy) _pawncamera))
  (bind _output_2 (Utilities|Array|Get(acopy) _pawncameraai))
  (bind _output_3 (Utilities|Array|Get(acopy) _pawncamera_2 1))
  (bind _output_4 (Utilities|Array|Get(acopy) _pawncameraai_2 2))
  (bind _output_5 (Utilities|Array|Get(acopy) _pawncameraai_3 1))
  (bind _output_6 (Utilities|Array|Get(acopy) _pawncamera_3 2))
  ;[1 1 1] Event tick (mengatur detikan UI, switch antara player dan AI, dan setting player atau AI ke start di level itu) --Margareth
  (Utilities|FlowControl|Sequence
    (:then_0
      (Utilities|FlowControl|Delay 1.0)
      (if (not (== (Math|Integer|%(Integer) (Variables|Default|Getstart) 2) 1))
        (if (== (Variables|Default|GetSeconds) 0.0)
          (if (== (Variables|Default|GetMinutes) 0.0)
            (Default|HidePause _pc_player)
            (Default|DisplayLose _pc_player)
            (else
              (Variables|Default|SetSeconds 59.0)
              (Variables|Default|SetMinutes (- (Variables|Default|GetMinutes) 1))))
          (else
            (Variables|Default|SetSeconds (- (Variables|Default|GetSeconds) 1.0))))))
    (:then_1
      (if (== (Variables|Default|Getstart) 0)
        (Game|Player|SetViewTargetwithBlend _returnvalue_2 _output 0.0 "VTBlend_Linear" 0.0 false)
        (Pawn|Possess _returnvalue_2 _output)
        (Variables|Default|SetTotalFinish 1)
        (CallFunction|ShowUIPlayer)
        (elif (== (Variables|Default|Getstart) 1)
          (Game|Player|SetViewTargetwithBlend _returnvalue_3 _output_2 0.0 "VTBlend_Linear" 0.0 false)
          (Pawn|Possess _returnvalue_3 _output_2)
          (Variables|Default|SetTotalFinish 2)
          (CallFunction|ShowUIAI)
          (elif (== (Variables|Default|Getstart) 2)
            (Game|Player|SetViewTargetwithBlend _returnvalue_4 _output_3 0.0 "VTBlend_Linear" 0.0 false)
            (Pawn|Possess _returnvalue_4 _output_3)
            (Variables|Default|SetTotalFinish 3)
            (CallFunction|ShowUIPlayer)
            (elif (== (Variables|Default|Getstart) 3)
              (Game|Player|SetViewTargetwithBlend _returnvalue_5 _output_5 0.0 "VTBlend_Linear" 0.0 false)
              (Pawn|Possess _returnvalue_5 _output_5)
              (Variables|Default|SetTotalFinish 4)
              (CallFunction|ShowUIAI)
              (elif (== (Variables|Default|Getstart) 4)
                (Game|Player|SetViewTargetwithBlend _returnvalue_6 _output_6 0.0 "VTBlend_Linear" 0.0 false)
                (Pawn|Possess _returnvalue_6 _output_6)
                (Variables|Default|SetTotalFinish 5)
                (CallFunction|ShowUIPlayer)
                (elif (== (Variables|Default|Getstart) 5)
                  (Game|Player|SetViewTargetwithBlend _returnvalue _output_4 0.0 "VTBlend_Linear" 0.0 false)
                  (Pawn|Possess _returnvalue _output_4)
                  (Variables|Default|SetTotalFinish 6)
                  (CallFunction|ShowUIAI))))))))))

(fn ConstructionScript)