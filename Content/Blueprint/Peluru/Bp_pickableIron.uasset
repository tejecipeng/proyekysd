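; Iron bullet pickup actor that unlocks a bullet type for the player character.
; Its Pickup event casts the other actor to Bp_Character, sets the third entry of that character's Bullets boolean array to true, then destroys the pickup.
; BeginPlay, overlap and Tick are disabled stubs, and the construction script only calls the parent.
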(event EventBeginPlay
  (|CallParentFunction) ; This node is disabled and will not be called.\nDrag off pins to build functionality.
)

(event Collision|EventActorBeginOverlap
  (params (OtherActor :type Actor%20Object%20Reference))
  (|CallParentFunction OtherActor) ; This node is disabled and will not be called.\nDrag off pins to build functionality.
)

(event EventTick
  (params (DeltaSeconds :type Float%20%28single-precision%29))
  (|CallParentFunction DeltaSeconds) ; This node is disabled and will not be called.\nDrag off pins to build functionality.
)

(event EventPickup
  (params (OtherActor :type Actor%20Object%20Reference))
  (bind _asbp_character (Utilities|Casting|CastToBp_Character OtherActor))
  (Utilities|Array|SetArrayElem (Variables|/Game/Blueprint/char/Bp_Character.Bp_Character_C|GetBullets _asbp_character) 2 true)
  (Actor|DestroyActor))

(fn ConstructionScript
  (|CallParentFunction))